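; Activatable environment volume that changes the player character's gravity while they stand inside its Box.
; The Activate/Deactivate event toggles ForceActivated.
; Every Tick it checks the player pawn's overlap and, if active, passes GravityChangeInput to BP_BodyChar's GravityScale.
; When inactive or not overlapped, it sets a hardcoded default gravity scale every frame, so each instance keeps writing to the player even from afar.
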(event `self.Activate/Deactivate`
  (if (`self.ForceActivated`)
    (set `self.ForceActivated` false)
    (else
      (set `self.ForceActivated` true))))

(event `self.ReceiveTick`
  (params (DeltaSeconds :type "Float (single-precision)"))
  (bind _returnvalue (`GameplayStatics.GetPlayerPawn` 0))
  (if (`PrimitiveComponent.IsOverlappingActor` (`self.Box`) _returnvalue)
    (if (`self.ForceActivated`)
      (bind _asbp_body_char (cast `/Game/Dynamic/Blueprints/Characters/BodyChar/BP_BodyChar` _returnvalue))
      (`/Game/Dynamic/Blueprints/Characters/BodyChar/BP_BodyChar.GravityScale` _asbp_body_char (`self.GravityChangeInput`))
      (else
        (bind _asbp_body_char_2 (cast `/Game/Dynamic/Blueprints/Characters/BodyChar/BP_BodyChar` _returnvalue :!label _label))
        (`/Game/Dynamic/Blueprints/Characters/BodyChar/BP_BodyChar.GravityScale` _asbp_body_char_2 1.75)))
    (else
      (goto _label))))

(fn `UserConstructionScript`
  (`parent.UserConstructionScript`))